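; BP_TurtlesController is the controller for the turtles game that sets up the spawn-button UI and links it to the nests in the level.
; On BeginPlay it creates a single WBP_SpawnButtons widget and adds it to the player screen.
; It then finds every BP_Nest actor, passes the widget to its Nest, and registers that Nest and its mode back with the widget.
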(event `self.ReceiveBeginPlay`
  (`self.CreateWidget`)
  (`self.Share Widget`))

(fn `CreateWidget`
  (bind _returnvalue (`|CreateWidget` "/Game/Turtles/UI/WBP_SpawnButtons.WBP_SpawnButtons_C"))
  (`UserWidget.AddToPlayerScreen` _returnvalue 0)
  (set `self.Widget` _returnvalue))

(fn `Share Widget`
  (bind _outactors (`GameplayStatics.GetAllActorsOfClass` "/Game/Turtles/Characters/Nest/BP_Nest.BP_Nest_C"))
  (for _array_element _outactors
    (bind (_nest _nest_2) (`/Game/Turtles/Characters/Nest/BP_Nest.Nest` _array_element))
    (`NestComponent.SetWidget` _nest_2 (`self.Widget`))
    (`/Game/Turtles/UI/WBP_SpawnButtons.SetNest` (`self.Widget`) _nest_2 (`NestComponent.GetMode` _nest_2))))

(fn `UserConstructionScript`)
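; BP_FinishGate is the finish gate actor that registers turtles reaching it.
; On overlap it looks for a TurtleComponent on the other actor and calls ReceiveFinish on it, leaving the turtle's finish handling to that component.
; For those turtles it also spawns a finish particle effect at the gate's transform and attaches the finish sound to that emitter.
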(event `self.ReceiveActorBeginOverlap`
  (params (OtherActor :type "Actor Object Reference"))
  (bind _returnvalue (`self.GetComponentByClass` OtherActor "/Script/Turtles.TurtleComponent"))
  ;[1 1 1] Delete Turtle
  (if (`KismetSystemLibrary.IsValid` _returnvalue)
    (`TurtleComponent.ReceiveFinish` _returnvalue)
    ;[1 1 1] VFX and SFX
    (bind _returnvalue_2 (`GameplayStatics.SpawnEmitterAtLocation` (`self.FinishEffect`) (`self.K2_GetActorLocation`) (`self.K2_GetActorRotation`) (`self.GetActorScale3D`)))
    (`GameplayStatics.SpawnSoundAttached` (`self.FinishSound`) _returnvalue_2 "None" (0.0 0.0 0.0) (struct) "KeepRelativeOffset" false 1.0 1.0 0.0 null null)))

(fn `UserConstructionScript`)